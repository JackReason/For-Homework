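; Destructible block actor that takes hits from BP_Moving_Ball and drops a bonus when destroyed.
; Each ball hit raises a hit counter, and while the count is below Live the CubeL mesh switches to the golden material.
; Otherwise the actor destroys itself, prints a message and spawns one of two random bonus cube types at CubeL's location.
; The weighted drop roll is set to always succeed.
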(event `self.ReceiveHit`
  (params (MyComp :type "PrimitiveComponent Object Reference") (Other :type "Actor Object Reference") (OtherComp :type "PrimitiveComponent Object Reference") (bSelfMoved :type Boolean) (HitLocation :type "Vector Structure") (HitNormal :type "Vector Structure") (NormalImpulse :type "Vector Structure") (Hit :type "HitResult Structure (by ref)"))
  (cast `/Game/BP_Moving_Ball` Other)
  (bind _result (`/Engine/EditorBlueprintResources/StandardMacros.IncrementInt` (`self.Hits`))
    (:`  `
      (if (> (`self.Live`) _result)
        (`PrimitiveComponent.SetMaterial` (`self.CubeL`) 0 "/Game/Old_BPs/BP_Golden.BP_Golden")
        (else
          (set `self.Location` (`SceneComponent.K2_GetComponentLocation` (`self.CubeL`)))
          (`self.K2_DestroyActor`)
          (`KismetSystemLibrary.PrintString` "Destroyed!" true true (struct :`G` 0.66 :`B` 1.0 :`A` 1.0) 20.0)
          (if (`KismetMathLibrary.RandomBoolWithWeight` 1.0)
            (switch `int` (`KismetMathLibrary.RandomInteger` 2)
              (:`0`
                (`|SpawnActorFromClass` "/Game/BP_Bonus_Cube.BP_Bonus_Cube_C" (`KismetMathLibrary.MakeTransform` (`self.Location`)) "AlwaysSpawn" "OverrideRootScale" null null))
              (:`1`
                (`|SpawnActorFromClass` "/Game/BP_Bonus_Cube2.BP_Bonus_Cube2_C" (`KismetMathLibrary.MakeTransform` (`self.Location`) (struct) (1.0 1.0 2.0)) "AlwaysSpawn" "OverrideRootScale" null null)))))))))

(fn `UserConstructionScript`)