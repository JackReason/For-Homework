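; BP_Pawn2 is a player pawn that slides sideways along world Y and keeps a moving ball in play.
; Two MoveRight axis handlers apply a fixed-step, swept world offset according to the input's sign, without delta-time scaling.
; BeginPlay spawns a half-scale BP_Moving_Ball at the capsule and binds its OnDead event, which loops back to spawn and bind a replacement.
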(event `InputAxis|MoveRight`
  (params (AxisValue :type "Float (single-precision)"))
  (if (< AxisValue 0.0)
    (`self.K2_AddActorWorldOffset` (0.0 -5.0 0.0) true)))

(event `InputAxis|MoveRight`
  (params (AxisValue :type "Float (single-precision)"))
  (if (> AxisValue 0.0)
    (`self.K2_AddActorWorldOffset` (0.0 5.0 0.0) true)))

(event `self.ReceiveBeginPlay`
  (bind _returnvalue (`|SpawnActorFromClass` "/Game/BP_Moving_Ball.BP_Moving_Ball_C" (`KismetMathLibrary.MakeTransform` (`SceneComponent.K2_GetComponentLocation` (`self.Capsule`)) (struct) (0.5 0.5 0.5)) "AlwaysSpawn" "OverrideRootScale" null null :!label _label))
  (bind _output_get (set `self.NewBall` _returnvalue))
  (add `/Game/BP_Moving_Ball.OnDead` _output_get (delegate `CustomEvent_0`)))

(event `CustomEvent_0`
  (goto _label))

(fn `UserConstructionScript`)