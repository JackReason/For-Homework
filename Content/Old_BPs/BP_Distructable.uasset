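; BP_Distructable is a destructible actor that breaks after repeated hits from BP_Moving_Ball.
; A hit counts when the ball's overlap with the actor ends, incrementing Hits and comparing it against Live.
; While Live is higher it prints the hit count on screen; otherwise it destroys the actor and prints a destroyed message.
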(event `self.ReceiveActorEndOverlap`
  (params (OtherActor :type "Actor Object Reference"))
  (cast `/Game/BP_Moving_Ball` OtherActor)
  (bind _result (`/Engine/EditorBlueprintResources/StandardMacros.IncrementInt` (`self.Hits`))
    (:`  `
      (if (> (`self.Live`) _result)
        (`KismetSystemLibrary.PrintString` (`KismetStringLibrary.Concat_StrStr` "Hits:" (`KismetStringLibrary.Conv_IntToString` _result)) true true (struct :`G` 0.66 :`B` 1.0 :`A` 1.0) 5.0)
        (else
          (`self.K2_DestroyActor`)
          (`KismetSystemLibrary.PrintString` "Destroyed!" true true (struct :`G` 0.66 :`B` 1.0 :`A` 1.0) 20.0))))))

(fn `UserConstructionScript`)