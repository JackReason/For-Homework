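; Child Blueprint actor, named as a destructible, that toggles the material of its CubeL component whenever an actor stops overlapping it.
; On each end overlap it increments the ChangeColor counter and uses its parity to alternate between the BP_Golden and BP_Shiny materials.
; Both branches then pass the event to the parent's end-overlap logic, and construction only runs the parent's script.
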(event `self.ReceiveActorEndOverlap`
  (params (OtherActor :type "Actor Object Reference"))
  (bind _output_get (set `self.ChangeColor` (stale _result)))
  (bind _result (`/Engine/EditorBlueprintResources/StandardMacros.IncrementInt` _output_get)
    (:`  `
      (if (== (mod _result 2) 1)
        (`PrimitiveComponent.SetMaterial` (`self.CubeL`) 0 "/Game/Old_BPs/BP_Golden.BP_Golden")
        (`parent.ReceiveActorEndOverlap` OtherActor)
        (else
          (`PrimitiveComponent.SetMaterial` (`self.CubeL`) 0 "/Game/Old_BPs/BP_Shiny.BP_Shiny")
          (`parent.ReceiveActorEndOverlap` OtherActor))))))

(fn `UserConstructionScript`
  (`parent.UserConstructionScript`))